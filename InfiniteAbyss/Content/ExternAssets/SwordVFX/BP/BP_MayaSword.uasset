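; Maya's sword actor, exposing controls for its glow colors, Niagara sword effect, trail density and electric charging effect.
; UpdateProperties runs on construction and color changes, assigning the chosen Niagara asset, pushing rate, speed and offset parameters, and tinting effects and blade/fuller emissive materials.
; Toggle events switch the main effect together with fuller visibility, or the charging effect on its own.
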(event `self.ReceiveBeginPlay`)

(event `/Game/ExternAssets/SwordVFX/BP/BPI_Sword.SetTrailDensity`
  (params (Density :type Integer))
  (`NiagaraComponent.SetVariableInt` (`self.NS_SwordEffectComp`) "User.TrailSpawnRate" Density))

(event `/Game/ExternAssets/SwordVFX/BP/BPI_Sword.SetSwordColors`
  (params (SwordColor :type "LinearColor Structure") (EffectColor :type "LinearColor Structure"))
  (set `self.SwordColor` SwordColor)
  (set `self.EffectColor` EffectColor)
  (`self.UpdateProperties`))

(event `/Game/ExternAssets/SwordVFX/BP/BPI_Sword.ToggleSwordEffect`
  (params (Enable :type Boolean))
  (bind _ns_swordeffectcomp (`self.NS_SwordEffectComp`))
  (bind _fuller (`self.Fuller`))
  (if Enable
    (`ActorComponent.Activate` _ns_swordeffectcomp true)
    (`SceneComponent.SetHiddenInGame` _fuller false false)
    (else
      (`ActorComponent.Deactivate` _ns_swordeffectcomp)
      (`SceneComponent.SetHiddenInGame` _fuller true false))))

(event `/Game/ExternAssets/SwordVFX/BP/BPI_Sword.ToggleChargingEffect`
  (params (Enable :type Boolean))
  (bind _ns_electricsword (`self.NS_ElectricSword`))
  (if Enable
    (`ActorComponent.Activate` _ns_electricsword false)
    (else
      (`ActorComponent.Deactivate` _ns_electricsword))))

(fn `UpdateProperties`
  (`NiagaraComponent.SetAsset` (`self.NS_SwordEffectComp`) (`self.SwordEffect `) true)
  (`NiagaraComponent.SetVariableLinearColor` (`self.NS_SwordEffectComp`) "User.MainColor" (`self.EffectColor`))
  (`NiagaraComponent.SetVariableLinearColor` (`self.NS_ElectricSword`) "User.MainColor" (`self.EffectColor`))
  (`MeshComponent.SetVectorParameterValueOnMaterials` (`self.Fuller`) "Emissive Color" (`KismetMathLibrary.Conv_LinearColorToVector` (`self.SwordColor`)))
  (`MeshComponent.SetVectorParameterValueOnMaterials` (`self.sword`) "Emissive Color" (`KismetMathLibrary.Conv_LinearColorToVector` (`self.SwordColor`)))
  (`NiagaraComponent.SetVariableFloat` (`self.NS_SwordEffectComp`) "User.Rate1" (`self.Rate1`))
  (`NiagaraComponent.SetVariableFloat` (`self.NS_SwordEffectComp`) "User.Rate2" (`self.Rate2`))
  (`NiagaraComponent.SetVariableFloat` (`self.NS_SwordEffectComp`) "User.Speed1" (`self.Speed1`))
  (`NiagaraComponent.SetVariableFloat` (`self.NS_SwordEffectComp`) "User.Speed2" (`self.Speed2`))
  (`NiagaraComponent.SetVariableFloat` (`self.NS_SwordEffectComp`) "User.MeshOffset1" (`self.MeshOffset1`)))

(fn `UserConstructionScript`
  (`self.UpdateProperties`))