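; Configurable light shaft (god ray) actor built from a static mesh with a dynamic material.
; The construction script creates the material from an animated instance or the master material, then pushes spotlight, size, color, brightness and fade distance settings into it.
; It optionally copies the Sun actor's rotation to the mesh's relative rotation.
; A seeded random stream sets a per-instance random material parameter.
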(fn `UserConstructionScript`
  (bind _staticmesh1 (`self.StaticMesh1`))
  (bind _dynamic_material (`self.Dynamic material`))
  ;[1 1 1] Setting Material Parameters
  (if (`self.Animated`)
    (bind _returnvalue (`PrimitiveComponent.CreateDynamicMaterialInstance` _staticmesh1 0 "/Game/LuosCaves/Materials/Extra_Prop_Instances/MI_godray_Animated.MI_godray_Animated"))
    (set `self.Dynamic material` _returnvalue)
    (else
      (bind _returnvalue_2 (`PrimitiveComponent.CreateDynamicMaterialInstance` _staticmesh1 0 "/Game/LuosCaves/Materials/Extra_Masters/M_godray_Master.M_godray_Master"))
      (set `self.Dynamic material` _returnvalue_2)))
  (if (`self.UseSun`)
    (`SceneComponent.K2_SetRelativeRotation` (`self.StaticMesh1`) (`self.K2_GetActorRotation` (`self.Sun`)) true))
  ;;[1 1 1] Pink
  (if (`self.SpotLight`)
    (`MaterialInstanceDynamic.SetScalarParameterValue` _dynamic_material "Spotlight" 1.0)
    (else
      (`MaterialInstanceDynamic.SetScalarParameterValue` _dynamic_material "Spotlight" 0.0)))
  (`MaterialInstanceDynamic.SetScalarParameterValue` _dynamic_material "1. Mesh width" (`self.1. Mesh Width`))
  (`MaterialInstanceDynamic.SetScalarParameterValue` _dynamic_material "2. Mesh Length" (`self.2. Mesh Length`))
  (`MaterialInstanceDynamic.SetVectorParameterValue` _dynamic_material "2. color" (`self.2. Color`))
  (`MaterialInstanceDynamic.SetScalarParameterValue` _dynamic_material "3. Brightness" (`self.3. Brightness`))
  (`MaterialInstanceDynamic.SetScalarParameterValue` _dynamic_material "5. fadedistance" (`self.5. FadeDistance`))
  (`MaterialInstanceDynamic.SetScalarParameterValue` _dynamic_material "6. random" (`KismetMathLibrary.RandomFloatInRangeFromStream` 0.0 100.0 (`self.RandomTime`))))